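; BP_HexGrid builds a hexagonal tile grid in its construction script, sized by Width and Height and spaced from the mesh bounds, Scale and Offset.
; A FlipFlop staggers alternate rows to form the hex layout.
; An Instanced flag selects either BP_Tile child actors or mesh instances.
; Instances get a random water or land height, which sets their Z position and is written to per-instance custom data.
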(event EventBeginPlay)

(event Collision|EventActorBeginOverlap
  (params (OtherActor :type Actor%20Object%20Reference)))

(event EventTick
  (params (DeltaSeconds :type Float%20%28single-precision%29)))

(fn ConstructionScript
  (bind _returnvalue (Math|Random|RandomFloatinRange -1.0 1.0))
  (Components|StaticMesh|SetStaticMesh (Variables|Default|GetInstancedStaticMesh) (Variables|GridOptions|GetTileMesh))
  (Variables|Default|SetRadius (* (.x (.max (StaticMesh|GetBoundingBox (Variables|GridOptions|GetTileMesh)))) (Variables|GridOptions|GetScale)))
  ;[1 1 1] Height
  (for _index (range 0 (- (Variables|GridOptions|GetHeight) 1))
    ;[1 1 1] Width
    (for _index_2 (range 0 (- (Variables|GridOptions|GetWidth) 1))
      (if (Variables|GridOptions|GetInstanced)
        ;[1 1 1] Siatka instancji
        (bind _returnvalue_2 (Components|InstancedStaticMesh|AddInstance (Variables|Default|GetInstancedStaticMesh) (Math|Transform|MakeTransform (Math|Vector|MakeVector (+ (* _index_2 (Variables|Default|GetRadius) 2.0) (* _index_2 (Variables|GridOptions|GetOffset)) (Variables|Default|GetRowOffset)) (+ (* (/ (* (Variables|Default|GetRadius) 2.0) (Math|Float|Sqrt 3.0)) 1.5 _index) (* _index (Variables|GridOptions|GetOffset))) 0.0) "0, 0, 0" (Math|Conversions|ToVector(Float) (Variables|GridOptions|GetScale))) false))
        (Variables|InstancedTile|SetInstancedIndex _returnvalue_2)
        ;[1 1 1] Fragment do losowego generowania wysokosci kafelkow, taki sam jak w BP_Tile
        (if (<= _returnvalue 0.0)
          (Variables|InstancedTile|SetTileHeight (Variables|InstancedTile|GetBaseWaterHeight))
          (else
            (Variables|InstancedTile|SetTileHeight (Math|Float|Clamp(Float) _returnvalue 0.1))))
        (Components|InstancedStaticMesh|UpdateInstanceTransform (Variables|Default|GetInstancedStaticMesh) (Variables|InstancedTile|GetInstancedIndex) (Math|Transform|MakeTransform (+ (.location (.OutInstanceTransform (Components|InstancedStaticMesh|GetInstanceTransform (Variables|Default|GetInstancedStaticMesh) (Variables|InstancedTile|GetInstancedIndex) true))) (Math|Vector|MakeVector 0.0 0.0 (+ (* (Variables|InstancedTile|GetTileHeight) (Variables|InstancedTile|GetTileHeightScale)) (Variables|InstancedTile|GetTileOffset)))) "0, 0, 0" "1.000000,1.000000,1.000000") false false false)
        (Components|InstancedStaticMesh|SetCustomDataValue (Variables|Default|GetInstancedStaticMesh) (Variables|InstancedTile|GetInstancedIndex) 0 (Variables|InstancedTile|GetTileHeight) true)
        (else
          (bind _returnvalue_3 (AddComponent|AddChildActorComponent false (Math|Transform|MakeTransform (Math|Vector|MakeVector (+ (* _index_2 (Variables|Default|GetRadius) 2.0) (* _index_2 (Variables|GridOptions|GetOffset)) (Variables|Default|GetRowOffset)) (+ (* (/ (* (Variables|Default|GetRadius) 2.0) (Math|Float|Sqrt 3.0)) 1.5 _index) (* _index (Variables|GridOptions|GetOffset))) 0.0) "0, 0, 0" (Math|Conversions|ToVector(Float) (Variables|GridOptions|GetScale)))))
          (ChildActorComponent|SetChildActorClass _returnvalue_3 "/Game/Mesh/BP_Tile.BP_Tile_C")
          (bind _asbp_tile (Utilities|Casting|CastToBP_Tile (Variables|/Script/Engine.ChildActorComponent|GetChildActor _returnvalue_3)))
          (Components|StaticMesh|SetStaticMesh (Variables|/Game/Mesh/BP_Tile.BP_Tile_C|GetStaticMesh _asbp_tile) (Variables|GridOptions|GetTileMesh)))))
    (Utilities|FlowControl|FlipFlop
      (:A
        ;[1 1 1] Co 2 rzad przesuwanie w lewo
        (Variables|Default|SetRowOffset (* (Variables|Default|GetRadius) -1.0)))
      (:B
        (Variables|Default|SetRowOffset 0.0)))))