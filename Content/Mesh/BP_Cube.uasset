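; BP_Cube is a static mesh Blueprint that randomizes its vertical placement and passes the random value to its materials.
; The construction script rolls a random Height from -1 to 1, then shifts the mesh in world Z by Height times HeightScale plus Offset.
; The same value sets the "Height" scalar material parameter, tying appearance to elevation.
; BeginPlay and the Random R and G OnRep functions are empty.
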(event EventBeginPlay)

(fn ConstructionScript
  (bind _staticmesh (Variables|Default|GetStaticMesh))
  (Variables|Default|SetHeight (Math|Random|RandomFloatinRange -1.0 1.0))
  (Transformation|SetWorldLocation _staticmesh (+ (Transformation|GetWorldLocation _staticmesh) (Math|Vector|MakeVector 0.0 0.0 (+ (* (Variables|Default|GetHeight) (Variables|Default|GetHeightScale)) (Variables|Default|GetOffset)))) false false)
  (Rendering|Material|SetScalarParameterValueonMaterials (Variables|Default|GetStaticMesh) "Height" (Variables|Default|GetHeight)))

(fn OnRepRandomG)

(fn OnRepRandomR)