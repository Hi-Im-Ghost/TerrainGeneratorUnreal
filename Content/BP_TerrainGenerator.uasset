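; Procedural terrain actor that builds a noise-based heightmap mesh with collision in its Construction Script.
; A configurable FastNoise wrapper sets the height of each vertex on a scaled X/Y grid, alongside scaled UVs.
; The grid is triangulated two triangles per cell, then normals and tangents are calculated before the ProceduralMesh section is created and given its material.
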(event EventBeginPlay)

(fn ConstructionScript
  (bind _returnvalue (Game|ConstructObjectfromClass "/Script/FastNoiseGenerator.FastNoiseWrapper"))
  (bind _output_get (Variables|Default|SetNoise _returnvalue))
  (Class|FastNoiseWrapper|SetupFastNoise _output_get (Variables|Noise|GetNoise%20Type) (Variables|Noise|GetSeed) (Variables|Noise|GetFrequency) (Variables|Noise|GetInterp) (Variables|Noise|GetFractaltype) (Variables|Noise|GetOctaves) (Variables|Noise|GetLacunarity) (Variables|Noise|GetGain) (Variables|Noise|GetCellular%20Jitter) (Variables|Noise|GetCellular%20Distance%20Function) (Variables|Noise|GetCellular%20Return%20Type))
  (CallFunction|SetVertices)
  (CallFunction|SetTraingles)
  (|CalculateNormalsandTangents)
  (Class|ProceduralMeshComponent|CreateMeshSectionLinearColor (Variables|Default|GetProceduralMesh) 0 (Variables|Default|GetVertices) (Variables|Default|GetTriangles) (Variables|Default|GetNormals) (Variables|Default|GetUV0) 0 0 0 0 (Variables|Default|GetTangents) true false)
  (Rendering|Material|SetMaterial (Variables|Default|GetProceduralMesh) 0 (Variables|Default|GetMaterial)))

(fn SetVertices
  (for _index (range 0 (Variables|Default|GetXSize))
    (LocalVariables|SetX _index)
    (for _index_2 (range 0 (Variables|Default|GetYSize))
      (LocalVariables|SetY _index_2)
      (Utilities|Array|Add (Variables|Default|GetVertices) (Math|Vector|MakeVector (* (LocalVariables|GetX) (Variables|Default|GetScale)) (* (LocalVariables|GetY) (Variables|Default|GetScale)) (* (Class|FastNoiseWrapper|GetNoise2D (Variables|Default|GetNoise) (+ (Math|Conversions|ToFloat(Integer) (LocalVariables|GetX)) 0.1) (+ (Math|Conversions|ToFloat(Integer) (LocalVariables|GetY)) 0.1)) (Variables|Default|GetZMultiplier))))
      (Utilities|Array|Add (Variables|Default|GetUV0) (Math|Vector2D|MakeVector2D (* (LocalVariables|GetX) (Variables|Default|GetUVScale)) (* (LocalVariables|GetY) (Variables|Default|GetUVScale)))))))

(fn SetTraingles
  (for _index (range 0 (- (Variables|Default|GetXSize) 1))
    (for _index_2 (range 0 (- (Variables|Default|GetYSize) 1))
      (Utilities|Array|Add (Variables|Default|GetTriangles) (LocalVariables|GetVertex))
      (Utilities|Array|Add (Variables|Default|GetTriangles) (+ (LocalVariables|GetVertex) 1))
      (Utilities|Array|Add (Variables|Default|GetTriangles) (+ (Variables|Default|GetYSize) (LocalVariables|GetVertex) 1))
      (Utilities|Array|Add (Variables|Default|GetTriangles) (+ (LocalVariables|GetVertex) 1))
      (Utilities|Array|Add (Variables|Default|GetTriangles) (+ (Variables|Default|GetYSize) (LocalVariables|GetVertex) 2))
      (Utilities|Array|Add (Variables|Default|GetTriangles) (+ (Variables|Default|GetYSize) (LocalVariables|GetVertex) 1))
      (Math|Integer|IncrementInt (LocalVariables|GetVertex)))
    (Math|Integer|IncrementInt (LocalVariables|GetVertex))))